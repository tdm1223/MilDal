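; Character Blueprint for the second player, driven by SendP2 movement and jump events rather than input bindings in its own graph.
; Move forward and right feed normalized world X and Y directions into movement input, so movement ignores facing and analog magnitude.
; An IsReverse flag, only read here, inverts both axes.
; Jumping resets the movement component's gravity scale to normal before calling Jump.
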(event `/Game/Blueprints/ControlsTransfer.Send_P2_Jump`
  (set `CharacterMovementComponent.GravityScale` 1.0 (`self.CharacterMovement`))
  (`self.Jump`))

(event `/Game/Blueprints/ControlsTransfer.Send_P2_Move_Right`
  (params (Axis_Value :type "Float (single-precision)"))
  (bind _returnvalue (`KismetMathLibrary.Normal` (`KismetMathLibrary.MakeVector` 0.0 Axis_Value)))
  (if (`self.bIsReverse`)
    (`self.AddMovementInput` (* _returnvalue -1.0))
    (else
      (`self.AddMovementInput` _returnvalue))))

(event `/Game/Blueprints/ControlsTransfer.Send_P2_Move_Forward`
  (params (Axis_Value :type "Float (single-precision)"))
  (bind _returnvalue (`KismetMathLibrary.Normal` (`KismetMathLibrary.MakeVector` Axis_Value)))
  (if (`self.bIsReverse`)
    (`self.AddMovementInput` (* _returnvalue -1.0))
    (else
      (`self.AddMovementInput` _returnvalue))))

(fn `UserConstructionScript`)