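; PlayerOne is a playable character that handles input for two players, moving and jumping itself and relaying the second player's controls.
; Its own axis inputs drive movement along fixed world X and Y axes, independent of camera or actor rotation.
; The "Two" inputs look up all PlayerTwo actors on each event and call their SendP2 move and jump events, so one input receiver controls both characters.
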(event `InputAction|Jump` :overrideparent false
  (params (Key :type "Key Structure"))
  ;[1 1 1] PlayerOneJump
  (:`Pressed`
    (`self.Jump`))
  (:`Released`
    (`self.StopJumping`)))

(event `InputAction|JumpTwo`
  (params (Key :type "Key Structure"))
  ;[1 1 1] PlayerTwoJump
  (:`Pressed`
    (bind _outactors (`GameplayStatics.GetAllActorsOfClass` "/Game/Blueprints/PlayerTwo.PlayerTwo_C"))
    (`self.Send_P2_Jump` _outactors)))

(event `InputAxis|MoveForwardTwo`
  (params (AxisValue :type "Float (single-precision)"))
  ;[1 1 1] PlayerTwoMove
  (bind _outactors (`GameplayStatics.GetAllActorsOfClass` "/Game/Blueprints/PlayerTwo.PlayerTwo_C"))
  (`self.Send_P2_Move_Forward` _outactors AxisValue))

(event `InputAxis|MoveForward` :overrideparent false
  (params (AxisValue :type "Float (single-precision)"))
  ;[1 1 1] PlayerOneMove
  (`self.AddMovementInput` (`KismetMathLibrary.Normal` (`KismetMathLibrary.MakeVector` AxisValue))))

(event `InputAxis|MoveRightTwo`
  (params (AxisValue :type "Float (single-precision)"))
  ;[1 1 1] PlayerTwoMove
  (bind _outactors (`GameplayStatics.GetAllActorsOfClass` "/Game/Blueprints/PlayerTwo.PlayerTwo_C"))
  (`self.Send_P2_Move_Right` _outactors AxisValue))

(event `InputAxis|MoveRight` :overrideparent false
  (params (AxisValue :type "Float (single-precision)"))
  ;[1 1 1] PlayerOneMove
  (`self.AddMovementInput` (`KismetMathLibrary.Normal` (`KismetMathLibrary.MakeVector` 0.0 AxisValue))))

(fn `UserConstructionScript`)